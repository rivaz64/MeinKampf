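; Behavior tree task that gives an Enemy pawn its current patrol location.
; It reads the path index from the blackboard, picks that entry from the enemy's PatrolPath points and converts it to world space with the path actor's transform.
; The result is written to the path point key, and the task fails if the pawn is not an Enemy or has no valid path.
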(event `self.ReceiveExecuteAI`
  (params (OwnerController :type "AIController Object Reference") (ControlledPawn :type "Pawn Object Reference"))
  (bind _asenemy (cast `/Game/Mara/Blueprints/AI/Enemy` ControlledPawn)
    (:`then`
      (bind _patrolpath (`/Game/Mara/Blueprints/AI/Enemy.PatrolPath` _asenemy)
        (:`then`
          (`BTFunctionLibrary.SetBlackboardValueAsVector` (`self.BB_PathPoint`) (`KismetMathLibrary.TransformLocation` (`Actor.GetTransform` _patrolpath) (`|GetArrayItem` (`/Game/Mara/Blueprints/AI/PathPoint_BP.PathPoints` _patrolpath) (`BTFunctionLibrary.GetBlackboardValueAsInt` (`self.BB_PathIndex`)))))
          (`self.FinishExecute` true))
        (:`else`
          (`self.FinishExecute` false :!label _label))))
    (:`CastFailed`
      (goto _label))))