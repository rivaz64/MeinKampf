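; Behavior tree task that advances an Enemy to the next point on its patrol path.
; It adds one to the path index in the Blackboard, wrapping by the number of PathPoints on the pawn's PatrolPath, then finishes successfully.
; It fails if the pawn is not an Enemy, and never calls FinishExecute if the PatrolPath is invalid.
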(event `self.ReceiveExecuteAI`
  (params (OwnerController :type "AIController Object Reference") (ControlledPawn :type "Pawn Object Reference"))
  (bind _bb_pathindex (`self.BB_PathIndex`))
  (bind _asenemy (cast `/Game/Mara/Blueprints/AI/Enemy` ControlledPawn)
    (:`then`
      (bind _patrolpath (`/Game/Mara/Blueprints/AI/Enemy.PatrolPath` _asenemy)
        (:`then`
          (`BTFunctionLibrary.SetBlackboardValueAsInt` _bb_pathindex (mod (+ (`BTFunctionLibrary.GetBlackboardValueAsInt` _bb_pathindex) 1) (`KismetArrayLibrary.Array_Length` (`/Game/Mara/Blueprints/AI/PathPoint_BP.PathPoints` _patrolpath))))
          (`self.FinishExecute` true))
        (:`else`)))
    (:`CastFailed`
      (`self.FinishExecute` false))))