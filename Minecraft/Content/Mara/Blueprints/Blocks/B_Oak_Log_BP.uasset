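; Oak log block actor that breaks into a collectible item drop when it is no longer alive.
; Tick polls IsAlive, which this graph never sets, rather than reacting to an event.
; Once false, it spawns the break particle effect and a single ItemDroped_BP carrying DropItemBlock with no collection delay, then destroys itself.
; The construction script is empty.
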(event `self.ReceiveTick`
  (params (DeltaSeconds :type "Float (single-precision)"))
  (bind _returnvalue (`self.K2_GetActorLocation`))
  (if (not (`self.isAlive`))
    (`NiagaraFunctionLibrary.SpawnSystemAtLocation` "/Game/Mara/Particles/BrokeBlock_PS.BrokeBlock_PS" _returnvalue)
    (bind _returnvalue_2 (`|SpawnActorFromClass` "/Game/Mara/Blueprints/Items/ItemDroped_BP.ItemDroped_BP_C" (`KismetMathLibrary.MakeTransform` _returnvalue) "Undefined" "OverrideRootScale" null null))
    (set `ItemDroped_CPP.Item` (`self.DropItemBlock`) _returnvalue_2)
    (set `ItemDroped_CPP.Count` 1 _returnvalue_2)
    (set `ItemDroped_CPP.TimeTillCollected` 0.0 _returnvalue_2)
    (`self.K2_DestroyActor`)))

(fn `UserConstructionScript`)