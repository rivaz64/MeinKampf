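; Crafting table block that opens the player's crafting UI and drops itself as an item when broken.
; Each Tick polls an OpenWidget flag, which adds the FirstPersonCharacter's CraftingWidget to the viewport, shows the mouse cursor and resets the flag.
; Tick also polls IsAlive; when false, the block plays a break particle effect, spawns a single dropped-item pickup and destroys itself.
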(event `self.ReceiveTick`
  (params (DeltaSeconds :type "Float (single-precision)"))
  (bind _returnvalue (`self.K2_GetActorLocation`))
  (if (`self.OpenWidget`)
    (bind _asfirst_person_character (cast `/Game/FirstPersonCPP/Blueprints/FirstPersonCharacter` (`GameplayStatics.GetPlayerCharacter` 0)))
    (`UserWidget.AddToViewport` (`/Game/FirstPersonCPP/Blueprints/FirstPersonCharacter.CraftingWidget` _asfirst_person_character) 0)
    (set `self.OpenWidget` false)
    (set `PlayerController.bShowMouseCursor` true (`GameplayStatics.GetPlayerController` 0)))
  (if (not (`self.isAlive`))
    (`NiagaraFunctionLibrary.SpawnSystemAtLocation` "/Game/Mara/Particles/BrokeBlock_PS.BrokeBlock_PS" _returnvalue)
    (bind _returnvalue_2 (`|SpawnActorFromClass` "/Game/Mara/Blueprints/Items/ItemDroped_BP.ItemDroped_BP_C" (`KismetMathLibrary.MakeTransform` _returnvalue) "Undefined" "OverrideRootScale" null null))
    (set `ItemDroped_CPP.Item` (`self.DropItemBlock`) _returnvalue_2)
    (set `ItemDroped_CPP.Count` 1 _returnvalue_2)
    (set `ItemDroped_CPP.TimeTillCollected` 0.0 _returnvalue_2)
    (`self.K2_DestroyActor`)))

(fn `UserConstructionScript`)