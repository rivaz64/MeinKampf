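; ItemDroped_BP is a dropped item pickup that holds an item and count and hands them to the FirstPersonCharacter.
; Once its tick-counted Timer runs out, it pops the mesh with a random upward impulse, then polls overlapping actors every Tick.
; When TimeTillCollected allows, Tick or begin-overlap adds it to the character, destroying it on success.
; Tick also merges it into overlapping drops of the same item within MaxStack.
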(event `self.ReceiveTick`
  (params (DeltaSeconds :type "Float (single-precision)"))
  (bind _item (`self.Item`))
  (if (> (`self.Timer`) 0)
    (set `self.Timer` (- (`self.Timer`) 1))
    (elif (`self.Fisic`)
      (if (<= (`self.TimeTillCollected`) 0.0)
        (for _array_element (`self.GetOverlappingActors` null)
          (bind _asfirst_person_character (cast `/Game/FirstPersonCPP/Blueprints/FirstPersonCharacter` _array_element)
            (:`then`
              (bind _returnvalue (`MinecraftCharacter.AddItem` _asfirst_person_character (`self.Item`) (`self.Count`)))
              (if _returnvalue
                (`self.K2_DestroyActor`)))
            (:`CastFailed`
              (bind _asitem_droped_bp (cast `/Game/Mara/Blueprints/ItemDroped_BP` _array_element))
              (bind _returnvalue_2 (+ (`ItemDroped_CPP.Count` _asitem_droped_bp) (`self.Count`)))
              (if (and (== (`ItemDroped_CPP.Item` _asitem_droped_bp) _item) (<= _returnvalue_2 (`.MaxStack` (defaults `Object` _item))))
                (set `ItemDroped_CPP.Count` _returnvalue_2 _asitem_droped_bp)
                (`self.K2_DestroyActor`))))))
      (else
        (`PrimitiveComponent.AddImpulseAtLocation` (`self.ItemMesh`) (`KismetMathLibrary.MakeVector` (`KismetMathLibrary.RandomFloatInRange` -100.0 100.0) (`KismetMathLibrary.RandomFloatInRange` -100.0 100.0) 100.0) (0.0 0.0 0.0) "None")
        (set `self.Fisic` true)))))

(event `self.ReceiveActorBeginOverlap`
  (params (OtherActor :type "Actor Object Reference"))
  (if (<= (`self.TimeTillCollected`) 0.0)
    (bind _asfirst_person_character (cast `/Game/FirstPersonCPP/Blueprints/FirstPersonCharacter` OtherActor))
    (bind _returnvalue (`MinecraftCharacter.AddItem` _asfirst_person_character (`self.Item`) (`self.Count`)))
    (if _returnvalue
      (`self.K2_DestroyActor`))))

(fn `UserConstructionScript`)